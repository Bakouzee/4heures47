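; DepotLegumeBP is the vegetable drop-off for the taste-room puzzle, opening the exit grille when the right five vegetables are deposited.
; Each overlapping LegumesBP has its value recorded, then is replaced by a copy spawned at its stored LegumePos.
; Tick polls for five deposits and compares them with the target list.
; A match destroys GrilleFinSalleGout; a mismatch clears the list and costs the player a chance, each with a sound.
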(event `self.CollisionComponent.OnComponentBeginOverlap`
  (params (OverlappedComponent :type "PrimitiveComponent Object Reference") (OtherActor :type "Actor Object Reference") (OtherComp :type "PrimitiveComponent Object Reference") (OtherBodyIndex :type Integer) (bFromSweep :type Boolean) (SweepResult :type "HitResult Structure (by ref)"))
  (bind _aslegumes_bp (cast `/Game/J-M/prefab/LegumesBP` OtherActor))
  (bind _legume (`/Game/J-M/prefab/LegumesBP.Legume` _aslegumes_bp))
  (`KismetArrayLibrary.Array_Add` (`self.ListAComparer`) _legume)
  (set `self.I` (+ (`self.I`) 1))
  (bind _returnvalue (`|SpawnActorFromClass` "/Game/J-M/prefab/LegumesBP.LegumesBP_C" (`/Game/J-M/prefab/LegumesBP.legumePos` _aslegumes_bp) "Undefined" "OverrideRootScale" null null))
  (set `/Game/J-M/prefab/LegumesBP.Legume` _legume _returnvalue)
  (`StaticMeshComponent.SetStaticMesh` (`/Game/J-M/prefab/LegumesBP.StaticMesh` _returnvalue) (`/Game/J-M/prefab/LegumesBP.MeshLegume` _aslegumes_bp))
  (`self.K2_DestroyActor` _aslegumes_bp))

(event `self.ReceiveTick`
  (params (DeltaSeconds :type "Float (single-precision)"))
  (bind _listacomparer (`self.ListAComparer`))
  (if (== (`self.I`) 5)
    (if (`KismetArrayLibrary.Array_Identical` (`self.ListATrouver`) _listacomparer)
      (set `self.I` 0)
      (`GameplayStatics.PlaySoundAtLocation` "/Game/SondEffect/S_StatueGood.S_StatueGood" (0.0 0.0 0.0) (struct) 1.0 1.0 0.0 null null null)
      (bind _returnvalue (`GameplayStatics.GetActorOfClass` "/Game/Assets/Props/Grille/grilleFinSalleGout.grilleFinSalleGout_C"))
      (`self.K2_DestroyActor` _returnvalue)
      (else
        (`KismetArrayLibrary.Array_Clear` _listacomparer)
        (set `self.sondefaite` true)
        (set `self.I` 0)
        (bind _asfirst_person_character (cast `/Game/FirstPersonBP/Blueprints/FirstPersonCharacter` (`GameplayStatics.GetPlayerPawn` 0)))
        (set `/Game/FirstPersonBP/Blueprints/FirstPersonCharacter.Chances` (- (`/Game/FirstPersonBP/Blueprints/FirstPersonCharacter.Chances` _asfirst_person_character) 1) _asfirst_person_character)
        (`GameplayStatics.PlaySoundAtLocation` "/Game/SondEffect/S_StatueWrong.S_StatueWrong" (0.0 0.0 0.0) (struct) 1.0 1.0 0.0 null null null)))))

(fn `UserConstructionScript`)